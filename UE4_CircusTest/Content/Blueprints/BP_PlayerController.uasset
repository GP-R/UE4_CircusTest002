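; Player controller that maps movement and look input to the player pawn according to the Mode held in BP_GameInstance.
; Main Mode uses standard movement input for forward and strafe.
; Cycle Mode nudges the pawn forward by setting its location without sweep or frame-time scaling, ignores backward input, and turns right/left input into actor roll.
; Turn and LookUp feed controller yaw and pitch identically in both modes.
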(event `InputAxis|MoveForward`
  (params (AxisValue :type "Float (single-precision)"))
  (bind _returnvalue (`GameplayStatics.GetPlayerPawn` 0))
  (bind _returnvalue_2 (`GameplayStatics.GetPlayerPawn` 0))
  (bind _asbp_game_instance (cast `/Game/Blueprints/BP_GameInstance` (`GameplayStatics.GetGameInstance`)))
  (switch `/Game/Blueprints/EMode` (`/Game/Blueprints/BP_GameInstance.Mode` _asbp_game_instance)
    (:`NewEnumerator3`
      (`Pawn.AddMovementInput` _returnvalue (`self.GetActorForwardVector` _returnvalue) AxisValue false))
    (:`NewEnumerator1`
      (if (> AxisValue 0.0)
        (`self.K2_SetActorLocation` _returnvalue_2 (+ (`self.K2_GetActorLocation` _returnvalue_2) (* (* (`self.GetActorForwardVector` _returnvalue_2) AxisValue) 1.0)) false false)))))

(event `InputAxis|MoveRight`
  (params (AxisValue :type "Float (single-precision)"))
  (bind _returnvalue (`GameplayStatics.GetPlayerPawn` 0))
  (bind _returnvalue_2 (`GameplayStatics.GetPlayerPawn` 0))
  (bind (_returnvalue_roll _returnvalue_pitch _returnvalue_yaw) (`KismetMathLibrary.BreakRotator` (`self.K2_GetActorRotation` _returnvalue_2)))
  (bind _asbp_game_instance (cast `/Game/Blueprints/BP_GameInstance` (`GameplayStatics.GetGameInstance`)))
  (switch `/Game/Blueprints/EMode` (`/Game/Blueprints/BP_GameInstance.Mode` _asbp_game_instance)
    (:`NewEnumerator3`
      (`Pawn.AddMovementInput` _returnvalue (`self.GetActorRightVector` _returnvalue) AxisValue false))
    (:`NewEnumerator1`
      (`self.K2_SetActorRotation` _returnvalue_2 (`KismetMathLibrary.MakeRotator` (+ _returnvalue_roll AxisValue) _returnvalue_pitch _returnvalue_yaw) false))))

(event `InputAxis|Turn`
  (params (AxisValue :type "Float (single-precision)"))
  (bind _asbp_game_instance (cast `/Game/Blueprints/BP_GameInstance` (`GameplayStatics.GetGameInstance`)))
  (switch `/Game/Blueprints/EMode` (`/Game/Blueprints/BP_GameInstance.Mode` _asbp_game_instance)
    (:`NewEnumerator3`
      _)
    (:`NewEnumerator1`
      _))
  (`self.AddYawInput` AxisValue))

(event `InputAxis|LookUp`
  (params (AxisValue :type "Float (single-precision)"))
  (bind _asbp_game_instance (cast `/Game/Blueprints/BP_GameInstance` (`GameplayStatics.GetGameInstance`)))
  (switch `/Game/Blueprints/EMode` (`/Game/Blueprints/BP_GameInstance.Mode` _asbp_game_instance)
    (:`NewEnumerator3`
      _)
    (:`NewEnumerator1`
      _))
  (`self.AddPitchInput` AxisValue))

(fn `UserConstructionScript`)