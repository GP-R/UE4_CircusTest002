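; BP_MaskHeadYellow is an interactable yellow mask pickup that adds its face entry to the mask selection UI.
; On BeginPlay it registers itself as YellowMask on BP_MainLvController.
; Interaction applies AddFaceImage to the WBP_SelectMask face color, appends it to FaceImageArray and makes that index current.
; The actor is then moved to a far-off location rather than hidden or destroyed.
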(event `self.ReceiveBeginPlay`
  (bind _asbp_main_lv_controller (cast `/Game/Blueprints/GameManager/BP_MainLvController` (`GameplayStatics.GetPlayerController` 0)))
  (set `/Game/Blueprints/GameManager/BP_MainLvController.YellowMask` self _asbp_main_lv_controller))

(event `self.Interaction`
  (bind _addfaceimage (`self.AddFaceImage`))
  (bind _asbp_main_lv_controller (cast `/Game/Blueprints/GameManager/BP_MainLvController` (`GameplayStatics.GetPlayerController` 0)))
  (bind _aswbp_select_mask (cast `/Game/Blueprints/Widget/WBP_SelectMask` (`MainPlayerController.SelectMaskUI` _asbp_main_lv_controller)))
  (`Image.SetColorAndOpacity` (`/Game/Blueprints/Widget/WBP_SelectMask.Face` _aswbp_select_mask) _addfaceimage)
  (bind _returnvalue (`KismetArrayLibrary.Array_Add` (`/Game/Blueprints/Widget/WBP_SelectMask.FaceImageArray` _aswbp_select_mask) _addfaceimage))
  (set `/Game/Blueprints/Widget/WBP_SelectMask.CurVisibleIndex` _returnvalue _aswbp_select_mask)
  (`self.SetActorHiddenInGame` false)
  (`self.K2_SetActorLocation` (99999.0 0.0 0.0)))

(fn `UserConstructionScript`)