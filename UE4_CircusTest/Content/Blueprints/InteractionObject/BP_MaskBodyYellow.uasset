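; BP_MaskBodyYellow is an interactable mask body that moves the player into mask selection.
; On Interaction it hides the player pawn and HUD, spawns and possesses a BP_SelectMaskPawn at the player's transform.
; A timeline interpolates that pawn to a fixed camera position and rotation.
; On arrival it shows the controller's mask selection UI and mouse cursor and records this body as the selected one.
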(event `self.ReceiveBeginPlay`
  (bind _asbp_main_lv_controller (cast `/Game/Blueprints/GameManager/BP_MainLvController` (`GameplayStatics.GetPlayerController` 0)))
  (set `self.PlayerController` _asbp_main_lv_controller))

(event `self.Interaction`
  (bind _returnvalue (`GameplayStatics.GetPlayerPawn` 0))
  (bind _playercontroller (`self.PlayerController`))
  (`self.SetActorHiddenInGame` (`GameplayStatics.GetPlayerPawn` 0) true)
  (`MainPlayerController.HidePlayerUI` (`self.PlayerController`))
  (bind _returnvalue_2 (`|SpawnActorFromClass` "/Game/Blueprints/Pawn/BP_SelectMaskPawn.BP_SelectMaskPawn_C" (`self.GetTransform` (`GameplayStatics.GetPlayerPawn` 0)) "Undefined" "OverrideRootScale" null null))
  (`Controller.Possess` (`GameplayStatics.GetPlayerController` 0) _returnvalue_2)
  (`Timeline|MovingCamera`
    (:`Update`
      (if (== (`self.CameraPosition(fix)`) (`self.K2_GetActorLocation` _returnvalue) :`ErrorTolerance` 5.0)
        (`TimelineComponent.Stop` (`self.MovingCamera`) :!label _label)
        (`self.K2_SetActorLocationAndRotation` (`GameplayStatics.GetPlayerPawn` 0) (`self.CameraPosition(fix)`) (struct :`Pitch` -10.0 :`Yaw` 90.0) false false)
        (`Widget.SetVisibility` (`MainPlayerController.SelectMaskUI` _playercontroller) "Visible")
        (set `PlayerController.bShowMouseCursor` true _playercontroller)
        (set `/Game/Blueprints/GameManager/BP_MainLvController.CurrentSelectedBody` 2 _playercontroller)
        (else
          (`self.K2_SetActorLocationAndRotation` _returnvalue (`KismetMathLibrary.VInterpTo` (`self.K2_GetActorLocation` _returnvalue) (`self.CameraPosition(fix)`) (`GameplayStatics.GetWorldDeltaSeconds`) 5.0) (`KismetMathLibrary.RInterpTo` (`self.K2_GetActorRotation` _returnvalue) (struct :`Pitch` -10.0 :`Yaw` 90.0) (`GameplayStatics.GetWorldDeltaSeconds`) 5.0) false false))))
    (:`Finished`
      (goto _label))))

(fn `UserConstructionScript`)