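; BP_CycleObject is an interactable placed object that switches the player over to a cycle pawn.
; On Interaction it spawns a BP_Cycle at its own transform, destroys the player's current pawn, has player controller 0 possess the new cycle, then destroys itself.
; A comment marks a sequence and mode change before self-destruction, but no nodes implement it.
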(event `self.Interaction`
  (bind _returnvalue (`|SpawnActorFromClass` "/Game/Blueprints/Pawn/BP_Cycle.BP_Cycle_C" (`self.GetTransform`) "Undefined" "OverrideRootScale" null null))
  (`self.K2_DestroyActor` (`GameplayStatics.GetPlayerPawn` 0))
  (`Controller.Possess` (`GameplayStatics.GetPlayerController` 0) _returnvalue)
  ;[1 1 1] 시퀀트실행 + 모드변경
  (`self.K2_DestroyActor`))

(fn `UserConstructionScript`
  (`parent.UserConstructionScript`))