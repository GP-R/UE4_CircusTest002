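; BP_Player is the player character, providing aim-based object interaction and stamina-limited sprinting.
; Each Tick it line-traces from a GameInstance-supplied screen point, storing the hit actor in BP_MainGameMode and toggling BP_InteractionObject highlights and the F-key prompt.
; The Interaction input calls Interaction on that stored actor.
; Run raises walk speed, with self-calling Delay events draining stamina until empty or regenerating it after release.
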(event `self.ReceiveBeginPlay`
  (bind _asbp_game_instance (cast `/Game/Blueprints/BP_GameInstance` (`GameplayStatics.GetGameInstance`)))
  (`|ExecutionSequence`
    (:`then_0`
      (`/Game/Blueprints/BP_GameInstance.SetMainMode` _asbp_game_instance))
    (:`then_1`
      (set `self.Screen Aim Position` (`/Game/Blueprints/BP_GameInstance.ScreenAimPosition` _asbp_game_instance)))
    (:`then_2`
      (set `self.Press FKey UI` (`/Game/Blueprints/BP_GameInstance.PressFKeyUI` _asbp_game_instance)))))

(event `self.ReceiveTick`
  (params (DeltaSeconds :type "Float (single-precision)"))
  (bind (_worldposition _worlddirection _returnvalue) (`GameplayStatics.DeprojectScreenToWorld` (`GameplayStatics.GetPlayerController` 0) (`self.Screen Aim Position`)))
  (`/Engine/EditorBlueprintResources/StandardMacros.IsValid` "BP_Player"
    (:`Is Valid`
      (if _returnvalue
        (bind (_outhit _returnvalue_2) (`KismetSystemLibrary.LineTraceSingle` :`Start` _worldposition :`End` (+ _worldposition (* _worlddirection (`self.InteractionRange`))) :`TraceChannel` "TraceTypeQuery3" :`DrawDebugType` "ForDuration"))
        (if _returnvalue_2
          (bind _asbp_main_game_mode (cast `/Game/Blueprints/BP_MainGameMode` (`GameplayStatics.GetGameMode`)))
          (bind _output_get (set `/Game/Blueprints/BP_MainGameMode.CurrentHitActor` (`.HitActor` (`GameplayStatics.BreakHitResult` _outhit)) _asbp_main_game_mode))
          (bind _asbp_interaction_object (cast `/Game/Blueprints/BP_InteractionObject` _output_get))
          (`/Game/Blueprints/BP_InteractionObject.StartHighlight` _asbp_interaction_object _output_get)
          (`Widget.SetVisibility` (`self.Press FKey UI`) "Visible")
          (else
            (`Widget.SetVisibility` (`self.Press FKey UI`) "Hidden")
            (bind _asbp_main_game_mode_2 (cast `/Game/Blueprints/BP_MainGameMode` (`GameplayStatics.GetGameMode`)))
            (bind _currenthitactor (`/Game/Blueprints/BP_MainGameMode.CurrentHitActor` _asbp_main_game_mode_2))
            (`/Engine/EditorBlueprintResources/StandardMacros.IsValid` _currenthitactor
              (:`Is Valid`
                (bind _asbp_interaction_object_2 (cast `/Game/Blueprints/BP_InteractionObject` _currenthitactor))
                (`/Game/Blueprints/BP_InteractionObject.EndHighlight` _asbp_interaction_object_2)
                (set `/Game/Blueprints/BP_MainGameMode.CurrentHitActor` null _asbp_main_game_mode_2)))))))))

(event `InputAction|Interaction`
  (params (Key :type "Key Structure"))
  (:`Pressed`
    (bind _asbp_main_game_mode (cast `/Game/Blueprints/BP_MainGameMode` (`GameplayStatics.GetGameMode`)))
    (bind _currenthitactor (`/Game/Blueprints/BP_MainGameMode.CurrentHitActor` _asbp_main_game_mode))
    (`/Engine/EditorBlueprintResources/StandardMacros.IsValid` _currenthitactor
      (:`Is Valid`
        (bind _asbp_interaction_object (cast `/Game/Blueprints/BP_InteractionObject` _currenthitactor))
        (`/Game/Blueprints/BP_InteractionObject.Interaction` _asbp_interaction_object)))))

(event `InputAction|Run`
  (params (Key :type "Key Structure"))
  (bind _charactermovement (`self.CharacterMovement`))
  (:`Pressed`
    (if (not (== (`MovementComponent.Velocity` _charactermovement) (0.0 0.0 0.0)))
      (set `CharacterMovementComponent.MaxWalkSpeed` 900.0 _charactermovement)
      (set `self.ShouldDrain` true)
      (`self.DrainStamina`)))
  (:`Released`
    (set `CharacterMovementComponent.MaxWalkSpeed` 600.0 _charactermovement)
    (set `self.ShouldDrain` false)
    (set `self.DesireStamina` 100.0)
    (`self.RegenStamina`)))

(event `DrainStamina`
  (if (`self.ShouldDrain`)
    (bind _output_get (set `self.Stamina` (`KismetMathLibrary.FClamp` (- (`self.Stamina`) 0.2) 0.0 (`self.MaxStamina`))))
    (if (== _output_get 0.0)
      (set `self.ShouldDrain` false)
      (set `CharacterMovementComponent.MaxWalkSpeed` 600.0 (`self.CharacterMovement`))
      (else
        (`KismetSystemLibrary.Delay` 0.01)
        (`self.DrainStamina`)))))

(event `RegenStamina`
  (if (`self.ShouldDrain`)
    _
    (elif (not (== (`self.Stamina`) (`self.DesireStamina`)))
      (set `self.Stamina` (`KismetMathLibrary.FClamp` (+ (`self.Stamina`) 0.1) 0.0 (`self.MaxStamina`)))
      (`KismetSystemLibrary.Delay` 0.01)
      (`self.RegenStamina`))))

(fn `UserConstructionScript`)