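; BP_CycleObject is an interactable world object that switches the player over to a BP_Cycle pawn.
; On Interaction it spawns BP_Cycle at its own transform, destroys the current player pawn and has the player controller possess the new one.
; It then changes the Mode enum on BP_GameInstance and destroys itself.
; Highlight start and end defer to the parent class, and its event graph holds only disabled stubs.
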(fn `EndHighlight`
  (`parent.EndHighlight`))

(fn `Interaction`
  (bind _returnvalue (`|SpawnActorFromClass` "/Game/Blueprints/BP_Cycle.BP_Cycle_C" (`self.GetTransform`) "Undefined" "OverrideRootScale" null null))
  (`self.K2_DestroyActor` (`GameplayStatics.GetPlayerPawn` 0))
  (`Controller.Possess` (`GameplayStatics.GetPlayerController` 0) _returnvalue)
  ;[1 1 1] 시퀀트실행 + 모드변경
  (bind _asbp_game_instance (cast `/Game/Blueprints/BP_GameInstance` (`GameplayStatics.GetGameInstance`)))
  (set `/Game/Blueprints/BP_GameInstance.Mode` "NewEnumerator1" _asbp_game_instance)
  (`self.K2_DestroyActor`))

(fn `StartHighlight`
  (params (HitActor :type "Actor Object Reference"))
  (`parent.StartHighlight` null))

(fn `UserConstructionScript`
  (`parent.UserConstructionScript`))