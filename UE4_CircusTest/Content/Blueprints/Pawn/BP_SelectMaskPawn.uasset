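; Pawn for a mask-matching selection step, where the player places red, mint or yellow masks on matching bodies.
; On BeginPlay it caches the main level controller and its mask selection widget.
; On SelectMask, if the visible face entry matches the controller's selected body, it moves that mask actor above the body with the same rotation.
; The entry then leaves the widget's array, and the face shows the previous one, wrapping around, or turns transparent when none remain.
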(event `self.ReceiveBeginPlay`
  (bind _asbp_main_lv_controller (cast `/Game/Blueprints/GameManager/BP_MainLvController` (`GameplayStatics.GetPlayerController` 0)))
  (bind _output_get (set `self.MainPlayerController` _asbp_main_lv_controller))
  (bind _aswbp_select_mask (cast `/Game/Blueprints/Widget/WBP_SelectMask` (`MainPlayerController.SelectMaskUI` _output_get)))
  (set `self.WBP_SelectMask` _aswbp_select_mask))

(event `InputAction|SelectMask`
  (params (Key :type "Key Structure"))
  (bind _mainplayercontroller (`self.MainPlayerController`))
  (bind _mainplayercontroller_2 (`self.MainPlayerController`))
  (bind _wbp_selectmask (`self.WBP_SelectMask`))
  (bind _wbp_selectmask_2 (`self.WBP_SelectMask`))
  (bind _wbp_selectmask_3 (`self.WBP_SelectMask`))
  (bind _mainplayercontroller_3 (`self.MainPlayerController`))
  (bind _wbp_selectmask_4 (`self.WBP_SelectMask`))
  (bind _wbp_selectmask_5 (`self.WBP_SelectMask`))
  (bind _wbp_selectmask_6 (`self.WBP_SelectMask`))
  (bind _faceimagearray (`/Game/Blueprints/Widget/WBP_SelectMask.FaceImageArray` _wbp_selectmask_5))
  (bind _redbody (`/Game/Blueprints/GameManager/BP_MainLvController.RedBody` _mainplayercontroller))
  (bind _mintbody (`/Game/Blueprints/GameManager/BP_MainLvController.MintBody` _mainplayercontroller_2))
  (bind _yellowbody (`/Game/Blueprints/GameManager/BP_MainLvController.YellowBody` _mainplayercontroller_3))
  (bind _faceimagearray_2 (`/Game/Blueprints/Widget/WBP_SelectMask.FaceImageArray` _wbp_selectmask_4))
  (bind _curvisibleindex (`/Game/Blueprints/Widget/WBP_SelectMask.CurVisibleIndex` _wbp_selectmask_4))
  (:`Pressed`
    (if (!= (`KismetArrayLibrary.Array_Length` (`/Game/Blueprints/Widget/WBP_SelectMask.FaceImageArray` (`self.WBP_SelectMask`))) 0)
      (if (and (== (`/Game/Blueprints/GameManager/BP_MainLvController.CurrentSelectedBody` (`self.MainPlayerController`)) 0) (== (`KismetArrayLibrary.Array_Find` (`/Game/Blueprints/Widget/WBP_SelectMask.FaceImageArray` _wbp_selectmask) (`self.RedMaskImage`)) (`/Game/Blueprints/Widget/WBP_SelectMask.CurVisibleIndex` _wbp_selectmask)))
        (`self.K2_SetActorLocationAndRotation` (`/Game/Blueprints/GameManager/BP_MainLvController.RedMask` _mainplayercontroller) (+ (`self.K2_GetActorLocation` _redbody) (0.0 0.0 240.0)) (`self.K2_GetActorRotation` _redbody) false false)
        (`KismetArrayLibrary.Array_Remove` _faceimagearray_2 _curvisibleindex :!label _label)
        (bind _result (`/Engine/EditorBlueprintResources/StandardMacros.DecrementInt` _curvisibleindex)
          (:`  `
            (if (== (`KismetArrayLibrary.Array_Length` _faceimagearray_2) 0)
              (`Image.SetColorAndOpacity` (`/Game/Blueprints/Widget/WBP_SelectMask.Face` (`self.WBP_SelectMask`)) (struct :`R` 1.0 :`G` 1.0 :`B` 1.0))
              (elif (== _result -1)
                (bind _output_get (set `/Game/Blueprints/Widget/WBP_SelectMask.CurVisibleIndex` (`KismetArrayLibrary.Array_LastIndex` _faceimagearray) _wbp_selectmask_5))
                (`Image.SetColorAndOpacity` (`/Game/Blueprints/Widget/WBP_SelectMask.Face` _wbp_selectmask_5) (`|GetArrayItem` _faceimagearray _output_get))
                (else
                  (`Image.SetColorAndOpacity` (`/Game/Blueprints/Widget/WBP_SelectMask.Face` _wbp_selectmask_6) (`|GetArrayItem` (`/Game/Blueprints/Widget/WBP_SelectMask.FaceImageArray` _wbp_selectmask_6) (`/Game/Blueprints/Widget/WBP_SelectMask.CurVisibleIndex` _wbp_selectmask_6))))))))
        (elif (and (== (`/Game/Blueprints/GameManager/BP_MainLvController.CurrentSelectedBody` (`self.MainPlayerController`)) 1) (== (`KismetArrayLibrary.Array_Find` (`/Game/Blueprints/Widget/WBP_SelectMask.FaceImageArray` _wbp_selectmask_2) (`self.MintMaskImage`)) (`/Game/Blueprints/Widget/WBP_SelectMask.CurVisibleIndex` _wbp_selectmask_2)))
          (`self.K2_SetActorLocationAndRotation` (`/Game/Blueprints/GameManager/BP_MainLvController.MintMask` _mainplayercontroller_2) (+ (`self.K2_GetActorLocation` _mintbody) (0.0 0.0 240.0)) (`self.K2_GetActorRotation` _mintbody) false false)
          (goto _label)
          (elif (and (== (`/Game/Blueprints/GameManager/BP_MainLvController.CurrentSelectedBody` (`self.MainPlayerController`)) 2) (== (`KismetArrayLibrary.Array_Find` (`/Game/Blueprints/Widget/WBP_SelectMask.FaceImageArray` _wbp_selectmask_3) (`self.YellowMaskImage`)) (`/Game/Blueprints/Widget/WBP_SelectMask.CurVisibleIndex` _wbp_selectmask_3)))
            (`self.K2_SetActorLocationAndRotation` (`/Game/Blueprints/GameManager/BP_MainLvController.YellowMask` _mainplayercontroller_3) (+ (`self.K2_GetActorLocation` _yellowbody) (0.0 0.0 240.0)) (`self.K2_GetActorRotation` _yellowbody) false false)
            (goto _label)))))))

(fn `UserConstructionScript`)