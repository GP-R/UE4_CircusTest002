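; Main level mode Blueprint that hands the level's three mask bodies to the player controller.
; On BeginPlay it casts player controller 0 to BP_MainLvController and stores it.
; It then finds the red, yellow and mint mask body actors with GetActorOfClass and writes them into that controller's RedBody, YellowBody and MintBody references.
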(event `self.ReceiveBeginPlay`
  (bind _asbp_main_lv_controller (cast `/Game/Blueprints/GameManager/BP_MainLvController` (`GameplayStatics.GetPlayerController` 0)))
  (set `self.MainLvController` _asbp_main_lv_controller)
  (`|ExecutionSequence`
    (:`then_1`
      (`|ExecutionSequence`
        (:`then_0`
          (bind _returnvalue (`GameplayStatics.GetActorOfClass` "/Game/Blueprints/InteractionObject/BP_MaskBodyRed.BP_MaskBodyRed_C"))
          (set `/Game/Blueprints/GameManager/BP_MainLvController.RedBody` _returnvalue (`self.MainLvController`)))
        (:`then_1`
          (bind _returnvalue_2 (`GameplayStatics.GetActorOfClass` "/Game/Blueprints/InteractionObject/BP_MaskBodyYellow.BP_MaskBodyYellow_C"))
          (set `/Game/Blueprints/GameManager/BP_MainLvController.YellowBody` _returnvalue_2 (`self.MainLvController`)))
        (:`then_2`
          (bind _returnvalue_3 (`GameplayStatics.GetActorOfClass` "/Game/Blueprints/InteractionObject/BP_MaskBodyMint.BP_MaskBodyMint_C"))
          (set `/Game/Blueprints/GameManager/BP_MainLvController.MintBody` _returnvalue_3 (`self.MainLvController`)))))))

(fn `UserConstructionScript`)