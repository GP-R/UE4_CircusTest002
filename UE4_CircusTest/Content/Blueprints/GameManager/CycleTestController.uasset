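; CycleTestController is a controller Blueprint with input axis events for movement and look, all of which do nothing.
; MoveForward, MoveRight, Turn and LookUp have empty bodies, and the construction script is empty.
; Unconnected leftover nodes would add yaw and pitch input, move the player pawn by movement input or direct location offset, and set its rotation, but none ever run.
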(event `InputAxis|MoveForward`
  (params (AxisValue :type "Float (single-precision)")))

(event `InputAxis|MoveRight`
  (params (AxisValue :type "Float (single-precision)")))

(event `InputAxis|Turn`
  (params (AxisValue :type "Float (single-precision)")))

(event `InputAxis|LookUp`
  (params (AxisValue :type "Float (single-precision)")))

(fn `UserConstructionScript`)