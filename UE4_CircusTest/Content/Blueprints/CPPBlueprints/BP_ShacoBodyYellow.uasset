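; Yellow Shaco body actor whose interaction opens the body selection view focused on it.
; Interaction hides the player pawn and UI, then spawns and possesses a BP_SelectShacoCamera at the player's transform.
; The MovingCamera timeline serves as a tick, interpolating the camera toward CameraPositionFix and snapping when close or finished.
; It then shows SelectUI and the cursor, with left and right buttons targeting the Mint and Red bodies' camera positions.
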(event `self.ReceiveBeginPlay`
  (bind _asbp_main_player_controller (cast `/Game/Blueprints/CPPBlueprints/BP_MainPlayerController` (`GameplayStatics.GetPlayerController` 0)))
  (set `self.PlayerController` _asbp_main_player_controller))

(event `self.Interaction`
  (bind _returnvalue (`GameplayStatics.GetPlayerPawn` 0))
  (bind _playercontroller (`self.PlayerController`))
  (bind _selectui (`/Game/Blueprints/CPPBlueprints/BP_MainPlayerController.SelectUI` _playercontroller))
  (`self.SetActorHiddenInGame` (`GameplayStatics.GetPlayerPawn` 0) true)
  (`MainPlayerController.HidePlayerUI` (`self.PlayerController`))
  (bind _returnvalue_2 (`|SpawnActorFromClass` "/Game/Blueprints/CPPBlueprints/BP_SelectShacoCamera.BP_SelectShacoCamera_C" (`self.GetTransform` (`GameplayStatics.GetPlayerPawn` 0)) "Undefined" "OverrideRootScale" null null))
  (`Controller.Possess` (`GameplayStatics.GetPlayerController` 0) _returnvalue_2)
  (`Timeline|MovingCamera`
    (:`Update`
      (if (== (`self.CameraPosition(fix)`) (`self.K2_GetActorLocation` _returnvalue) :`ErrorTolerance` 5.0)
        (`TimelineComponent.Stop` (`self.MovingCamera`) :!label _label)
        (`self.K2_SetActorLocationAndRotation` (`GameplayStatics.GetPlayerPawn` 0) (`self.CameraPosition(fix)`) (struct :`Pitch` -10.0 :`Yaw` 90.0) false false)
        (`Widget.SetVisibility` _selectui "Visible")
        (set `PlayerController.bShowMouseCursor` true _playercontroller)
        (set `/Game/Blueprints/CPPBlueprints/WBP_SelectShaco.LeftButtonTarget` (`/Game/Blueprints/CPPBlueprints/BP_ShacoBodyMint.CameraPosition(fix)` (`/Game/Blueprints/CPPBlueprints/BP_MainPlayerController.MintBody` _playercontroller)) _selectui)
        (set `/Game/Blueprints/CPPBlueprints/WBP_SelectShaco.RightButtonTarget` (`/Game/Blueprints/CPPBlueprints/BP_ShacoBodyRed.CameraPosition(fix)` (`/Game/Blueprints/CPPBlueprints/BP_MainPlayerController.RedBody` _playercontroller)) _selectui)
        (else
          (`self.K2_SetActorLocationAndRotation` _returnvalue (`KismetMathLibrary.VInterpTo` (`self.K2_GetActorLocation` _returnvalue) (`self.CameraPosition(fix)`) (`GameplayStatics.GetWorldDeltaSeconds`) 5.0) (`KismetMathLibrary.RInterpTo` (`self.K2_GetActorRotation` _returnvalue) (struct :`Pitch` -10.0 :`Yaw` 90.0) (`GameplayStatics.GetWorldDeltaSeconds`) 5.0) false false))))
    (:`Finished`
      (goto _label))))

(fn `UserConstructionScript`)