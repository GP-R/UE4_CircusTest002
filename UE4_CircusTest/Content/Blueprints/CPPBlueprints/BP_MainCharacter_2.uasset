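; Main character Blueprint that adds stamina-limited sprinting through the Run input.
; Pressing Run while moving raises walk speed and starts draining stamina, dropping back to normal speed when it empties.
; Releasing Run restores normal speed and starts regeneration toward the desired stamina level, at a slower rate than the drain.
; Drain and regen are self-calling events with short Delays, gated by the ShouldDrain flag instead of using Tick.
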(event `InputAction|Run`
  (params (Key :type "Key Structure"))
  (bind _charactermovement (`self.CharacterMovement`))
  (:`Pressed`
    (if (not (== (`MovementComponent.Velocity` _charactermovement) (0.0 0.0 0.0)))
      (set `CharacterMovementComponent.MaxWalkSpeed` 900.0 _charactermovement)
      (set `self.ShouldDrain` true)
      (`self.DrainStamina`)))
  (:`Released`
    (set `CharacterMovementComponent.MaxWalkSpeed` 600.0 _charactermovement)
    (set `self.ShouldDrain` false)
    (set `self.DesireStamina` 100.0)
    (`self.RegenStamina`)))

(event `DrainStamina`
  (if (`self.ShouldDrain`)
    (bind _output_get (set `self.Stamina` (`KismetMathLibrary.FClamp` (- (`self.Stamina`) 0.2) 0.0 (`self.MaxStamina`))))
    (if (== _output_get 0.0)
      (set `self.ShouldDrain` false)
      (set `CharacterMovementComponent.MaxWalkSpeed` 600.0 (`self.CharacterMovement`))
      (else
        (`KismetSystemLibrary.Delay` 0.01)
        (`self.DrainStamina`)))))

(event `RegenStamina`
  (if (`self.ShouldDrain`)
    _
    (elif (not (== (`self.Stamina`) (`self.DesireStamina`)))
      (set `self.Stamina` (`KismetMathLibrary.FClamp` (+ (`self.Stamina`) 0.1) 0.0 (`self.MaxStamina`)))
      (`KismetSystemLibrary.Delay` 0.01)
      (`self.RegenStamina`))))

(fn `UserConstructionScript`)