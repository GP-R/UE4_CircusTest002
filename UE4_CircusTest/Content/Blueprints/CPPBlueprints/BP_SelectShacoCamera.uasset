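; Blueprint for the Shaco selection camera that handles the SelectMask input on the mask/face selection UI.
; BeginPlay caches the BP_MainPlayerController, whose SelectUI holds the face array and visible index.
; Each press removes the current array entry and decrements the index, wrapping to the last entry at -1.
; The Face widget is then tinted with that entry's color, or made transparent once the array is empty.
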(event `self.ReceiveBeginPlay`
  (bind _asbp_main_player_controller (cast `/Game/Blueprints/CPPBlueprints/BP_MainPlayerController` (`GameplayStatics.GetPlayerController` 0)))
  (set `self.MainPlayerController` _asbp_main_player_controller))

(event `InputAction|SelectMask`
  (params (Key :type "Key Structure"))
  (bind _selectui (`/Game/Blueprints/CPPBlueprints/BP_MainPlayerController.SelectUI` (`self.MainPlayerController`)))
  (bind _selectui_2 (`/Game/Blueprints/CPPBlueprints/BP_MainPlayerController.SelectUI` (`self.MainPlayerController`)))
  (bind _selectui_3 (`/Game/Blueprints/CPPBlueprints/BP_MainPlayerController.SelectUI` (`self.MainPlayerController`)))
  (bind _faceimagearray (`/Game/Blueprints/CPPBlueprints/WBP_SelectShaco.FaceImageArray` _selectui_2))
  (bind _faceimagearray_2 (`/Game/Blueprints/CPPBlueprints/WBP_SelectShaco.FaceImageArray` _selectui))
  (bind _curvisibleindex (`/Game/Blueprints/CPPBlueprints/WBP_SelectShaco.CurVisibleIndex` _selectui))
  (:`Pressed`
    (if (!= (`KismetArrayLibrary.Array_Length` (`/Game/Blueprints/CPPBlueprints/WBP_SelectShaco.FaceImageArray` (`/Game/Blueprints/CPPBlueprints/BP_MainPlayerController.SelectUI` (`self.MainPlayerController`)))) 0)
      (`KismetArrayLibrary.Array_Remove` _faceimagearray_2 _curvisibleindex)
      (bind _result (`/Engine/EditorBlueprintResources/StandardMacros.DecrementInt` _curvisibleindex)
        (:`  `
          (if (== (`KismetArrayLibrary.Array_Length` _faceimagearray_2) 0)
            (`Image.SetColorAndOpacity` (`/Game/Blueprints/CPPBlueprints/WBP_SelectShaco.Face` (`/Game/Blueprints/CPPBlueprints/BP_MainPlayerController.SelectUI` (`self.MainPlayerController`))) (struct :`R` 1.0 :`G` 1.0 :`B` 1.0))
            (elif (== _result -1)
              (bind _output_get (set `/Game/Blueprints/CPPBlueprints/WBP_SelectShaco.CurVisibleIndex` (`KismetArrayLibrary.Array_LastIndex` _faceimagearray) _selectui_2))
              (`Image.SetColorAndOpacity` (`/Game/Blueprints/CPPBlueprints/WBP_SelectShaco.Face` _selectui_2) (`|GetArrayItem` _faceimagearray _output_get))
              (else
                (`Image.SetColorAndOpacity` (`/Game/Blueprints/CPPBlueprints/WBP_SelectShaco.Face` _selectui_3) (`|GetArrayItem` (`/Game/Blueprints/CPPBlueprints/WBP_SelectShaco.FaceImageArray` _selectui_3) (`/Game/Blueprints/CPPBlueprints/WBP_SelectShaco.CurVisibleIndex` _selectui_3)))))))))))

(fn `UserConstructionScript`)