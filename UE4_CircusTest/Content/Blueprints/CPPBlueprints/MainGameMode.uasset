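; MainGameMode is a game mode Blueprint that sets up the main player controller's Shaco selection UI and body references at BeginPlay.
; It creates a WBP_SelectShaco widget, stores it as the controller's SelectUI, and adds it to the viewport hidden.
; It then finds the red, yellow and mint Shaco body actors by class and assigns them to the controller.
; Setup stops if the BP_MainPlayerController cast fails.
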(event `self.ReceiveBeginPlay`
  (bind _playercontroller (`self.PlayerController`))
  (bind _asbp_main_player_controller (cast `/Game/Blueprints/CPPBlueprints/BP_MainPlayerController` (`GameplayStatics.GetPlayerController` 0)))
  (set `self.PlayerController` _asbp_main_player_controller)
  (`|ExecutionSequence`
    (:`then_0`
      (bind _returnvalue (`|CreateWidget` "/Game/Blueprints/CPPBlueprints/WBP_SelectShaco.WBP_SelectShaco_C" _playercontroller))
      (bind _output_get (set `/Game/Blueprints/CPPBlueprints/BP_MainPlayerController.SelectUI` _returnvalue _playercontroller))
      (`UserWidget.AddToViewport` _output_get 0)
      (`Widget.SetVisibility` _output_get "Hidden"))
    (:`then_1`
      (`|ExecutionSequence`
        (:`then_0`
          (bind _returnvalue_2 (`GameplayStatics.GetActorOfClass` "/Game/Blueprints/CPPBlueprints/BP_ShacoBodyRed.BP_ShacoBodyRed_C"))
          (set `/Game/Blueprints/CPPBlueprints/BP_MainPlayerController.RedBody` _returnvalue_2 (`self.PlayerController`)))
        (:`then_1`
          (bind _returnvalue_3 (`GameplayStatics.GetActorOfClass` "/Game/Blueprints/CPPBlueprints/BP_ShacoBodyYellow.BP_ShacoBodyYellow_C"))
          (set `/Game/Blueprints/CPPBlueprints/BP_MainPlayerController.YellowBody` _returnvalue_3 (`self.PlayerController`)))
        (:`then_2`
          (bind _returnvalue_4 (`GameplayStatics.GetActorOfClass` "/Game/Blueprints/CPPBlueprints/BP_ShacoBodyMint.BP_ShacoBodyMint_C"))
          (set `/Game/Blueprints/CPPBlueprints/BP_MainPlayerController.MintBody` _returnvalue_4 (`self.PlayerController`)))))))

(fn `UserConstructionScript`)